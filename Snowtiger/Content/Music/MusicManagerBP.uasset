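; Music manager Blueprint that plays a tracklist as 2D sounds and switches which track is audible.
; After a short delay on BeginPlay, it creates and starts every track muted, then raises the track at SongIndex to MusVolume.
; ChangeMusicTo mutes the current track and unmutes the requested one, an instant switch without restarting playback or crossfading.
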(event Custom|Change%20Music%20To
  (params (SongIndexToPlay :type Integer))
  (bind _music_references (Variables|Default|GetMusic%20References))
  (bind _output (Utilities|Array|Get(acopy) _music_references SongIndexToPlay))
  (Audio|Components|Audio|SetVolumeMultiplier (Variables|Default|GetCurrent%20Music%20Reference) 0.0 :!class /Script/Engine.AudioComponent)
  (Audio|Components|Audio|SetVolumeMultiplier _output (Variables|Default|GetMusVolume) :!class /Script/Engine.AudioComponent)
  (Variables|Default|SetCurrent%20Music%20Reference _output))

(event EventBeginPlay
  (bind _songindex (Variables|Default|GetSongIndex))
  (bind _music_references (Variables|Default|GetMusic%20References))
  (bind _output (Utilities|Array|Get(acopy) _music_references _songindex))
  (Utilities|FlowControl|Delay 0.6)
  (for _array_element (Variables|Default|GetTracklist)
    (bind _returnvalue (Audio|CreateSound2D _array_element 1.0 1.0 0.0 0))
    (Utilities|Array|Add (Variables|Default|GetMusic%20References) _returnvalue)
    (Audio|Components|Audio|SetVolumeMultiplier _returnvalue 0.0 :!class /Script/Engine.AudioComponent)
    (Audio|Components|Audio|Play _returnvalue 0.0))
  (Audio|Components|Audio|SetVolumeMultiplier _output (Variables|Default|GetMusVolume) :!class /Script/Engine.AudioComponent)
  (Variables|Default|SetCurrent%20Music%20Reference _output))

(fn ConstructionScript)